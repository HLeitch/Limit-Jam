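; BP_Lava_Top is a lava actor that the player raises and lowers with input actions, and that kills the player on contact.
; Holding Raise Lava or Lower Lava opens a gate that loops on a short Delay, offsetting the actor's Z until MaxHeight or MinHeight.
; BoxCollider overlap sets Alive to false on a FirstPersonCharacter.
; ChangeSpeed and StopMovement set CurrentSpeed, which the movement loops do not read.
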(event OnComponentBeginOverlap(BoxCollider)
  (params (OverlappedComponent :type Primitive%20Component%20Object%20Reference) (OtherActor :type Actor%20Object%20Reference) (OtherComp :type Primitive%20Component%20Object%20Reference) (OtherBodyIndex :type Integer) (bFromSweep :type Boolean) (SweepResult :type Hit%20Result%20Structure%20%28by%20ref%29))
  (CallFunction|CollisionwithPlayer OtherActor))

(event EventBeginPlay)

(event EventTick
  (params (DeltaSeconds :type Float%20%28single-precision%29)))

(event Input|ActionEvents|InputActionLowerLava
  (params (Key :type Key%20Structure :default "None"))
  (:Pressed
    (Utilities|FlowControl|Sequence
      (:then_0
        (goto _label Open))
      (:then_1
        (Utilities|FlowControl|Gate true :!label _label
          (:Exit
            (if (< (Variables|Default|GetminHeight) (.z (Transformation|GetWorldLocation (Variables|Default|GetDefaultSceneRoot))))
              (Transformation|AddActorWorldOffset (Math|Vector|MakeVector 0.0 0.0 (Variables|Default|GetLowerSpeed)))
              (Utilities|FlowControl|Delay 0.01)
              (goto _label)))))))
  (:Released
    (goto _label Close)))

(event Input|ActionEvents|InputActionRaiseLava
  (params (Key :type Key%20Structure :default "None"))
  (:Pressed
    (Utilities|FlowControl|Sequence
      (:then_0
        (goto _label Open))
      (:then_1
        (Utilities|FlowControl|Gate true :!label _label
          (:Exit
            (if (> (Variables|Default|GetmaxHeight) (.z (Transformation|GetWorldLocation (Variables|Default|GetDefaultSceneRoot))))
              (Transformation|AddActorWorldOffset (Math|Vector|MakeVector 0.0 0.0 (Variables|Default|GetRaise%20Speed)))
              (Utilities|FlowControl|Delay 0.01)
              (goto _label)))))))
  (:Released
    (goto _label Close)))

(fn ConstructionScript)

(fn ChangeSpeed
  (params (speed :type Float%20%28single-precision%29))
  (Variables|Default|SetcurrentSpeed speed))

(fn StopMovement
  (CallFunction|ChangeSpeed 0.0))

(fn CollisionwithPlayer
  (params (Object :type Object%20Object%20Reference))
  (bind _asfirst_person_character (Utilities|Casting|CastToFirstPersonCharacter Object))
  (Variables|/Game/FirstPersonBP/Blueprints/FirstPersonCharacter.FirstPersonCharacter_C|SetAlive _asfirst_person_character false))